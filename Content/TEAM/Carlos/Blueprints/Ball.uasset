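; Ball actor that scores goals when it overlaps a GoalDetecter.
; Its overlap event checks the detector's Porteria1 flag to pick the goal, then increments Marcador1 or Marcador2 on that detector.
; The new count is written to the matching score text in the HUD held by player 0's BP_ThirdPersonCharacter.
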(event OnComponentBeginOverlap(Ball)
  (params (OverlappedComponent :type Primitive%20Component%20Object%20Reference) (OtherActor :type Actor%20Object%20Reference) (OtherComp :type Primitive%20Component%20Object%20Reference) (OtherBodyIndex :type Integer) (bFromSweep :type Boolean) (SweepResult :type Hit%20Result%20Structure%20%28by%20ref%29))
  (bind _asgoal_detecter (Utilities|Casting|CastToGoalDetecter OtherActor))
  (if (Variables|/Game/TEAM/Carlos/Blueprints/GoalDetecter.GoalDetecter_C|GetPorteria1 _asgoal_detecter)
    (bind _result (Math|Integer|IncrementInt (Variables|/Game/TEAM/Carlos/Blueprints/GoalDetecter.GoalDetecter_C|GetMarcador1 _asgoal_detecter))
      (:%20%20
        (bind _asbp_third_person_character (Utilities|Casting|CastToBP_ThirdPersonCharacter (Game|GetPlayerCharacter 0)))
        (Rendering|Components|TextRender|SetText (Variables|/Game/TEAM/Carlos/Widgets/GameHud.GameHud_C|GetNumberMarcador1 (Variables|/Game/ThirdPerson/Blueprints/BP_ThirdPersonCharacter.BP_ThirdPersonCharacter_C|GetHUD _asbp_third_person_character)) (Utilities|Text|ToText(Integer) _result))))
    (else
      (bind _result_2 (Math|Integer|IncrementInt (Variables|/Game/TEAM/Carlos/Blueprints/GoalDetecter.GoalDetecter_C|GetMarcador2 _asgoal_detecter))
        (:%20%20
          (bind _asbp_third_person_character_2 (Utilities|Casting|CastToBP_ThirdPersonCharacter (Game|GetPlayerCharacter 0)))
          (Rendering|Components|TextRender|SetText (Variables|/Game/TEAM/Carlos/Widgets/GameHud.GameHud_C|GetNumberMarcador2 (Variables|/Game/ThirdPerson/Blueprints/BP_ThirdPersonCharacter.BP_ThirdPersonCharacter_C|GetHUD _asbp_third_person_character_2)) (Utilities|Text|ToText(Integer) _result_2)))))))

(fn ConstructionScript)